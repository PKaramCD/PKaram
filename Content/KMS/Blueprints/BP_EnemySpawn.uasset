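; Enemy spawner actor that creates a BP_EnemyBase at its SpawnEnemyPosition component.
; BeginPlay spawns the first enemy through the SpawnEnemy function and sets HasEnemy.
; Tick polls that flag and, when it is false, waits on a short Delay before spawning again and setting it back to true.
; Nothing in this Blueprint clears HasEnemy, and a loose SpawnActor node in the event graph never runs.
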(event `self.ReceiveBeginPlay`
  (`self.SpawnEnemy`)
  (set `self.HasEnemy` true))

(event `self.ReceiveTick`
  (params (DeltaSeconds :type "Float (single-precision)"))
  (if (not (`self.HasEnemy`))
    (`KismetSystemLibrary.Delay` 3.0)
    (`self.SpawnEnemy`)
    (set `self.HasEnemy` true)))

(event `CustomEvent`)

(fn `SpawnEnemy`
  (bind (_returnvalue_location _returnvalue_rotation) (`KismetMathLibrary.BreakTransform` (`SceneComponent.K2_GetComponentToWorld` (`self.SpawnEnemyPosition`))))
  (`|SpawnActorFromClass` "/Game/KMS/Blueprints/BP_EnemyBase.BP_EnemyBase_C" (`KismetMathLibrary.MakeTransform` _returnvalue_location _returnvalue_rotation) "Undefined" "MultiplyWithRoot" null null))

(fn `UserConstructionScript`)