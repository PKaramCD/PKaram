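; Player character with mouse click-to-move and a basic melee-style attack.
; Holding left mouse opens a Tick gate that moves toward the pawn under the cursor or the clicked point, walking slower for nearby points.
; A collision component flags tagged enemies or neutrals, but targets come from GetActorOfClass rather than the overlapped actor.
; Q applies damage only for regular enemies; incoming damage drains Health, destroying the player on a hit after depletion.
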(event `Key|LeftMouseButton`
  (params (Key :type "Key Structure"))
  ;[1 1 1] Click To Move - Gorak_Ver
)

(event `self.ReceiveBeginPlay`
  (set `PlayerController.bShowMouseCursor` true (`GameplayStatics.GetPlayerController` 0)))

(event `self.ReceiveTick`
  (params (DeltaSeconds :type "Float (single-precision)"))
  ;[1 1 1] ClickMove and Clicked Actor Connect Tick
  (`/Engine/EditorBlueprintResources/StandardMacros.Gate` true :!label _label
    (:`Exit`
      (bind _clickedactor (`self.GetClickedActor`))
      (`/Engine/EditorBlueprintResources/StandardMacros.IsValid` _clickedactor
        (:`Is Valid`
          (`self.MoveToActor` _clickedactor))
        (:`Is Not Valid`
          (`self.MoveToClickedPoint`))))))

(event `Key|LeftMouseButton`
  (params (Key :type "Key Structure"))
  ;[1 1 1] ClickMove and Clicked Actor Connect Tick
  (:`Pressed`
    (goto _label :!via `Open`))
  (:`Released`
    (goto _label :!via `Close`)))

(event `self.ReceiveActorBeginOverlap`
  (params (OtherActor :type "Actor Object Reference"))
  (if (`self.IsEnemy`)
    (set `self.CanAttack` true)
    (elif (`self.IsNeutralEnemy`)
      (set `self.CanAttack` true))))

(event `self.TargetCheckCollision_P.OnComponentBeginOverlap`
  (params (OverlappedComponent :type "PrimitiveComponent Object Reference") (OtherActor :type "Actor Object Reference") (OtherComp :type "PrimitiveComponent Object Reference") (OtherBodyIndex :type Integer) (bFromSweep :type Boolean) (SweepResult :type "HitResult Structure (by ref)"))
  (if (`self.ActorHasTag` OtherActor "Enemy")
    (set `self.IsEnemy` true)
    (set `self.IsNeutralEnemy` false)
    (bind _returnvalue (`GameplayStatics.GetActorOfClass` "/Game/KMS/Blueprints/BP_EnemyBase.BP_EnemyBase_C"))
    (bind _output_get (set `self.Target` _returnvalue))
    (`KismetSystemLibrary.PrintString` (`KismetSystemLibrary.GetDisplayName` _output_get))
    (elif (`self.ActorHasTag` OtherActor "NEnemy")
      (set `self.IsEnemy` false)
      (set `self.IsNeutralEnemy` true)
      (bind _returnvalue_2 (`GameplayStatics.GetActorOfClass` "/Game/KMS/Blueprints/BP_NeutralEnemyBase.BP_NeutralEnemyBase_C"))
      (bind _output_get_2 (set `self.Target` _returnvalue_2))
      (`KismetSystemLibrary.PrintString` (`KismetSystemLibrary.GetDisplayName` _output_get_2)))))

(event `self.TargetCheckCollision_P.OnComponentEndOverlap`
  (params (OverlappedComponent :type "PrimitiveComponent Object Reference") (OtherActor :type "Actor Object Reference") (OtherComp :type "PrimitiveComponent Object Reference") (OtherBodyIndex :type Integer))
  (set `self.IsEnemy` false)
  (set `self.IsNeutralEnemy` false)
  (set `self.CanAttack` false))

(event `self.ReceiveAnyDamage`
  (params (Damage :type "Float (single-precision)") (DamageType :type "DamageType Object Reference") (InstigatedBy :type "Controller Object Reference") (DamageCauser :type "Actor Object Reference"))
  ;[1 1 1] Take Damage
  (if (> (`self.Health`) 0.0)
    (set `self.Health` (- (`self.Health`) Damage))
    (`KismetSystemLibrary.PrintString` "Damaged!!!")
    (else
      (`self.K2_DestroyActor`))))

(event `Key|Q`
  (params (Key :type "Key Structure"))
  (:`Pressed`
    (if (`self.CanAttack`)
      (if (`self.IsEnemy`)
        (bind _returnvalue (`GameplayStatics.GetActorOfClass` "/Game/KMS/Blueprints/BP_EnemyBase.BP_EnemyBase_C"))
        (cast `Character` _returnvalue)
        (`GameplayStatics.ApplyDamage` null 20.0)))))

(fn `GetClickedActor`
  (returns (ClickedActor :type "Actor Object Reference"))
  (return (`.HitActor` (`GameplayStatics.BreakHitResult` (`PlayerController.GetHitResultUnderCursorForObjects` (`GameplayStatics.GetPlayerController` 0) (`|MakeArray` "ObjectTypeQuery3" :!type "EObjectTypeQuery Enum") true)))))

(fn `GetDestionationToMove`
  (returns (Destination :type "Vector Structure"))
  (return (`.Location` (`GameplayStatics.BreakHitResult` (`PlayerController.GetHitResultUnderCursorByChannel` (`GameplayStatics.GetPlayerController` 0) "TraceTypeQuery1" true)))))

(fn `MoveToActor`
  (params (MoveToActor :type "Actor Object Reference"))
  (`AIBlueprintHelperLibrary.SimpleMoveToActor` (`GameplayStatics.GetPlayerController` 0) MoveToActor))

(fn `MoveToClickedPoint`
  (locals (MoveDestination :type "Vector Structure"))
  (bind _charactermovement (`self.CharacterMovement`))
  (bind _destination (`self.GetDestionationToMove`))
  (set `local.MoveDestination` _destination)
  (if (> (`KismetMathLibrary.VSize` (- (`local.MoveDestination`) (`self.K2_GetActorLocation`))) 150.0)
    (set `CharacterMovementComponent.MaxWalkSpeed` 600.0 _charactermovement)
    (else
      (set `CharacterMovementComponent.MaxWalkSpeed` 150.0 _charactermovement)))
  (`AIBlueprintHelperLibrary.SimpleMoveToLocation` (`GameplayStatics.GetPlayerController` 0) (`local.MoveDestination`)))

(fn `UserConstructionScript`)